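; BP_GDD2GameMode is a game mode that creates and connects the game's button, story and effect managers.
; Its construction script constructs a ButtonManager object owned by the game mode.
; BeginPlay finds the first StoryManager and EffectManager actors, cross-registers the story and button managers, then registers the effect manager with the story manager.
; Getters expose the button and effect managers.
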(event `self.ReceiveBeginPlay`
  (bind _buttonmanager (`self.buttonManager`))
  (bind _outactors (`GameplayStatics.GetAllActorsOfClass` "/Script/GDD2.StoryManager"))
  (bind _output (`|GetArrayItem` _outactors))
  (`ButtonManager.RegisterStoryManager` _buttonmanager _output)
  (`StoryManager.RegisterButtonManager` _output _buttonmanager)
  (bind _outactors_2 (`GameplayStatics.GetAllActorsOfClass` "/Script/GDD2.EffectManager"))
  (bind _output_get (set `self.effectManager` (`|GetArrayItem` _outactors_2)))
  (`StoryManager.RegisterEffectManager` _output _output_get))

(fn `GetButtonManger`
  (returns (ButtonManager :type "ButtonManager Object Reference"))
  (return (`self.buttonManager`)))

(fn `GetEffectManager`
  (returns (EffectManager :type "EffectManager Object Reference"))
  (return (`self.effectManager`)))

(fn `UserConstructionScript`
  (`parent.UserConstructionScript`)
  (bind _returnvalue (`|GenericCreateObject` "/Script/GDD2.ButtonManager" self))
  (set `self.buttonManager` _returnvalue))