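; A smoke effect actor that drives a Niagara particle system and can be switched on and off.
; Init copies lifetime, spawn rate, sprite size and cone shape settings into the system's user parameters, then deactivates it unless it is initially active.
; Activate restores the spawn rate and, given a positive active time, deactivates after that delay.
; Deactivate sets the spawn rate to zero, and both events call their parent versions.
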(event `self.ReceiveBeginPlay`)

(event `self.Activate`
  (params (activeTime :type "Float (single-precision)"))
  (`parent.Activate` activeTime)
  (`NiagaraComponent.SetVariableFloat` (`self.SmokeParticelSystem`) "User.SpawnRate" (`self.spawnRate`))
  (`/Engine/EditorBlueprintResources/StandardMacros.CompareFloat` activeTime
    (:`>`
      (`KismetSystemLibrary.Delay` activeTime)
      (`self.Deactivate`))))

(event `self.Deactivate`
  (`parent.Deactivate`)
  (`NiagaraComponent.SetVariableFloat` (`self.SmokeParticelSystem`) "User.SpawnRate" 0.0))

(fn `Init`
  (`NiagaraComponent.SetVariableFloat` (`self.SmokeParticelSystem`) "User.LifeTimeMax" (`self.lifeTimeMax`))
  (`NiagaraComponent.SetVariableFloat` (`self.SmokeParticelSystem`) "User.SpawnRate" (`self.spawnRate`))
  (`NiagaraComponent.SetVariableFloat` (`self.SmokeParticelSystem`) "User.SpriteSize" (`self.spriteSize`))
  (`NiagaraComponent.SetVariableFloat` (`self.SmokeParticelSystem`) "User.ConeAngleMin" (`self.coneAngelMin`))
  (`NiagaraComponent.SetVariableFloat` (`self.SmokeParticelSystem`) "User.ConeAngleMax" (`self.coneAngleMax`))
  (`NiagaraComponent.SetVariableVec3` (`self.SmokeParticelSystem`) "User.ConeAxis" (`self.coneAxis`))
  (set `self.SpawnRateOriginal` (`self.spawnRate`))
  (if (not (`self.InitiallyActive`))
    (`self.Deactivate`)))

(fn `UserConstructionScript`)