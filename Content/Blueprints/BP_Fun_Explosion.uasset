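; BP_Fun_Explosion is an actor that plays a just-for-fun explosion effect with sound when its button function is called.
; FunExplosionButtonPressed sets a Launch flag if the cooldown since the last play has passed, and Tick consumes that flag.
; Tick moves the actor to a random point near its starting origin, plays a trigger sound, then after a delay activates the explosion particles and sound.
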(event `self.ReceiveBeginPlay`
  (set `self.origin` (`self.K2_GetActorLocation`)))

(event `self.ReceiveTick`
  (params (DeltaSeconds :type "Float (single-precision)"))
  (if (`self.launch`)
    (set `self.last_played_timestamp` (`KismetSystemLibrary.GetGameTimeInSeconds`))
    (set `self.launch` false)
    (`self.K2_SetActorLocation` (+ (`self.origin`) (* (* (`KismetMathLibrary.RandomUnitVector`) 100.0) (`KismetMathLibrary.RandomFloatInRange` 0.0 1.0))))
    (`/Game/Blueprints/BP_SFXManger.PlaySound` (`self.SFXManager`) "outdoor_explosion_trigger")
    (`KismetSystemLibrary.Delay` 3.0)
    (`ActorComponent.Activate` (`self.ExplosionParticles`) true)
    (`/Game/Blueprints/BP_SFXManger.PlaySound` (`self.SFXManager`) "outdoor_explosion")))

(fn `FunExplosionButtonPressed`
  (if (> (- (`KismetSystemLibrary.GetGameTimeInSeconds`) (`self.last_played_timestamp`)) 4.0)
    (set `self.launch` true)))

(fn `UserConstructionScript`)