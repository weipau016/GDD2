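; BP_EffectManager is a level-wide effects controller for smoke registration, camera fades and scene lighting.
; On BeginPlay it registers every SmokeEffect and caches all Light actors with their original intensities.
; Fade events spawn black or white camera-fade actors, while light events call the parent, then set or restore intensity and color across all lights.
; BlinkLight loops delayed visibility toggles until a timer clears its flag, then applies the reset color.
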(event `self.ReceiveBeginPlay`
  (bind _outactors (`GameplayStatics.GetAllActorsOfClass` "/Script/GDD2.SmokeEffect"))
  (for _array_element _outactors
    (`self.RegisterSmokeEffect` _array_element))
  (bind _outactors_2 (`GameplayStatics.GetAllActorsOfClass` "/Script/Engine.Light"))
  (bind _output_get (set `self.Lights` _outactors_2))
  (for (_array_element_2 _array_index) _output_get
    (`KismetArrayLibrary.Array_Set` (`self.OriginalLightIntensities`) _array_index (`LightComponentBase.Intensity` (`Light.LightComponent` _array_element_2)) true)))

(event `self.ActivateFadeToBlack`
  (params (fadeDuration :type "Float (single-precision)"))
  (`|SpawnActorFromClass` "/Game/Blueprints/BP_CameraFadeToBlack.BP_CameraFadeToBlack_C" (`self.GetTransform`) "Undefined" "OverrideRootScale" null fadeDuration false null))

(event `self.ActivateFadeToWhite`
  (params (fadeDuration :type "Float (single-precision)"))
  (`|SpawnActorFromClass` "/Game/Blueprints/BP_CameraFadeToWhite.BP_CameraFadeToWhite_C" (`self.GetTransform`) "Undefined" "OverrideRootScale" null fadeDuration false null))

(event `self.SetLightIntensity`
  (params (intensity :type "Float (single-precision)"))
  (`parent.SetLightIntensity` intensity)
  (for _array_element (`self.Lights`)
    (`LightComponent.SetIntensity` (`Light.LightComponent` _array_element) intensity)))

(event `self.ResetLightIntensity`
  (`parent.ResetLightIntensity`)
  (for (_array_element _array_index) (`self.Lights`)
    (`LightComponent.SetIntensity` (`Light.LightComponent` _array_element) (`|GetArrayItem` (`self.OriginalLightIntensities`) _array_index))))

(event `self.SetLightColor`
  (params (color :type "LinearColor Structure"))
  (`parent.SetLightColor` color)
  (for _array_element (`self.Lights`)
    (`LightComponent.SetLightColor` (`Light.LightComponent` _array_element) color true)))

(event `self.BlinkLight`
  (params (color :type "LinearColor Structure") (frequency :type "Float (single-precision)") (duration :type "Float (single-precision)") (resetColor :type "LinearColor Structure"))
  (`parent.BlinkLight` color frequency duration resetColor)
  (set `self.BlinkLights` true)
  (`self.SetLightColor` color)
  (`KismetSystemLibrary.K2_SetTimer` null "StopLightBlinking" duration)
  (if (`self.BlinkLights`) :!label _label
    (`KismetSystemLibrary.Delay` frequency)
    (`self.ToggleLights`)
    (`KismetSystemLibrary.Delay` (`self.LightBlinkOnTime`))
    (`self.ToggleLights`)
    (goto _label)
    (else
      (`self.SetLightColor` resetColor))))

(fn `StopLightBlinking`
  (set `self.BlinkLights` false))

(fn `ToggleLights`
  (for _array_element (`self.Lights`)
    (`SceneComponent.ToggleVisibility` (`Light.LightComponent` _array_element) false))
  (return))

(fn `UserConstructionScript`)